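; MagicStoneBP is an interactable stone that switches the game between DayLevel and NightLevel1.
; Its Collision overlap with BP_FirstPersonCharacter enables input and shows a WBP_InteractText prompt, both undone on exit.
; Pressing E in range saves the player's location and rotation to BP_GameInstance, then opens NightLevel1 from DayLevel, or DayLevel from any other level.
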(event OnComponentBeginOverlap(Collision)
  (params (OverlappedComponent :type Primitive%20Component%20Object%20Reference) (OtherActor :type Actor%20Object%20Reference) (OtherComp :type Primitive%20Component%20Object%20Reference) (OtherBodyIndex :type Integer) (bFromSweep :type Boolean) (SweepResult :type Hit%20Result%20Structure%20%28by%20ref%29))
  (bind _returnvalue (Game|GetPlayerController 0))
  (Utilities|Casting|CastToBP_FirstPersonCharacter OtherActor)
  (Variables|Default|SetCanInteract true)
  (Input|EnableInput _returnvalue)
  (bind _returnvalue_2 (UserInterface|CreateWidget "/Game/Blueprints/WBP_InteractText.WBP_InteractText_C" _returnvalue))
  (UserInterface|Viewport|AddtoViewport _returnvalue_2 0)
  (Variables|Default|SetInteractWidget _returnvalue_2))

(event OnComponentEndOverlap(Collision)
  (params (OverlappedComponent :type Primitive%20Component%20Object%20Reference) (OtherActor :type Actor%20Object%20Reference) (OtherComp :type Primitive%20Component%20Object%20Reference) (OtherBodyIndex :type Integer))
  (Utilities|Casting|CastToBP_FirstPersonCharacter OtherActor)
  (Variables|Default|SetCanInteract false)
  (Input|DisableInput (Game|GetPlayerController 0))
  (Widget|RemovefromParent (Variables|Default|GetInteractWidget)))

(event EventBeginPlay)

(event Collision|EventActorBeginOverlap
  (params (OtherActor :type Actor%20Object%20Reference)))

(event EventTick
  (params (DeltaSeconds :type Float%20%28single-precision%29)))

(event Input|KeyboardEvents|E
  (params (Key :type Key%20Structure :default "None"))
  (bind _returnvalue (Game|GetPlayerCharacter 0))
  (:Pressed
    (if (Variables|Default|GetCanInteract)
      (Widget|RemovefromParent (Variables|Default|GetInteractWidget))
      (bind _asbp_game_instance (Utilities|Casting|CastToBP_GameInstance (Game|GetGameInstance)))
      (Variables|/Game/Blueprints/BP_GameInstance.BP_GameInstance_C|SetSavedPlayerLocation _asbp_game_instance (Transformation|GetActorLocation _returnvalue))
      (Variables|/Game/Blueprints/BP_GameInstance.BP_GameInstance_C|SetSavedPlayerRotation _asbp_game_instance (Transformation|GetActorRotation _returnvalue))
      (bind _returnvalue_2 (Game|GetCurrentLevelName true))
      (if (Utilities|Enum|Equal(Enum) _returnvalue_2 "DayLevel")
        (Game|OpenLevel(byName) "NightLevel1")
        (else
          (Game|OpenLevel(byName) "DayLevel"))))))

(fn ConstructionScript)